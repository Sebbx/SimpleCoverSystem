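; Test cover manager actor that registers covers and both teams' AI characters inside its box at BeginPlay, then assigns covers to them.
; FindCoverForCharacter narrows candidates in stages: unreserved, enemy distance, protected yaw arcs, firing angle and range on any target, then nearest.
; Each character holds one reservation, replaced when another free cover is reserved.
; TakeReservedCovers sends characters through their AI controllers to reserved covers or default locations.
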(event Custom|ReserveCover
  (params (CoverToReserve :type BP%20Test%20Cover%20Base%20Object%20Reference) (AICharacter :type BP%20AI%20Base%20Object%20Reference))
  (Utilities|IsValid CoverToReserve
    (:Is%20Valid
      (if (Variables|/Game/Blueprints/BP_TestCoverBase.BP_TestCoverBase_C|GetbIsReserved CoverToReserve)
        (Development|PrintString "Cover is already reserved" true true "(R=1.000000,G=0.000000,B=0.149158,A=1.000000)")
        (else
          (CallFunction|DeleteReservation AICharacter true)
          (bind _output_get (Variables|/Game/AI/BP_AIBase.BP_AIBase_C|SetReservedCover AICharacter CoverToReserve))
          (Utilities|IsValid _output_get
            (:Is%20Valid
              (Variables|/Game/Blueprints/BP_TestCoverBase.BP_TestCoverBase_C|SetbIsReserved _output_get true)
              (Development|PrintString "Reservation successful" true true "(R=0.000000,G=1.000000,B=0.262904,A=1.000000)"))))))))

(event Custom|DeleteReservation
  (params (TargetAICharacter :type BP%20AI%20Base%20Object%20Reference) (bCalledByReservation :type Boolean))
  (Utilities|IsValid (Variables|/Game/AI/BP_AIBase.BP_AIBase_C|GetReservedCover TargetAICharacter)
    (:Is%20Valid
      (Variables|/Game/Blueprints/BP_TestCoverBase.BP_TestCoverBase_C|SetbIsReserved (Variables|/Game/AI/BP_AIBase.BP_AIBase_C|GetReservedCover TargetAICharacter) false)
      (Variables|/Game/AI/BP_AIBase.BP_AIBase_C|SetReservedCover TargetAICharacter 0)
      (Development|PrintString "Reservation deleted" true true "(R=0.000000,G=1.000000,B=0.262904,A=1.000000)"))
    (:Is%20Not%20Valid
      (if (not bCalledByReservation)
        (Development|PrintString "Character has no reservation" true true "(R=1.000000,G=0.000000,B=0.149158,A=1.000000)")))))

(event Custom|TakeReservedCovers
  (for _array_element (Variables|Default|GetAllAICharacters)
    (Utilities|IsValid (Variables|/Game/AI/BP_AIBase.BP_AIBase_C|GetReservedCover _array_element)
      (:Is%20Valid
        (bind _asaic_aicharacter (Utilities|Casting|CastToAIC_AICharacter (AI|GetAIController _array_element)))
        (Default|SetStateasGotoCover _asaic_aicharacter (Transformation|GetWorldLocation (Variables|/Game/Blueprints/BP_TestCoverBase.BP_TestCoverBase_C|GetCoverPosition (Variables|/Game/AI/BP_AIBase.BP_AIBase_C|GetReservedCover _array_element)))))
      (:Is%20Not%20Valid
        (Development|PrintString (Utilities|String|Append (Utilities|GetDisplayName _array_element) ": Has no reserved cover") true true "(R=1.000000,G=0.000000,B=0.041135,A=1.000000)")
        (bind _asaic_aicharacter_2 (Utilities|Casting|CastToAIC_AICharacter (AI|GetAIController _array_element)))
        (Default|SetStateasGotoCover _asaic_aicharacter_2 (Variables|/Game/AI/BP_AIBase.BP_AIBase_C|GetDefaultLocation _array_element))))))

(event Custom|FindAndReserveCover
  (params (TargetEnemy :type BP%20AI%20Base%20Object%20Reference) (GivenCharacter :type BP%20AI%20Base%20Object%20Reference))
  (bind _bestcover (CallFunction|FindCoverforCharacter TargetEnemy (select (Variables|/Game/AI/BP_AIBase.BP_AIBase_C|GetbIsEnemy GivenCharacter) (Variables|Default|GetEnemyTeamCharacters) (Variables|Default|GetPlayerTeamCharacters)) GivenCharacter))
  (CallFunction|ReserveCover _bestcover GivenCharacter))

(event Custom|FindCoverAndReserveForAllCharactersInTeam
  (params (TargetTeam :type Array%20of%20BP%20AI%20Base%20Object%20References) (OpossiteTeam :type Array%20of%20BP%20AI%20Base%20Object%20References))
  (for _array_element TargetTeam
    (bind _bestcover (CallFunction|FindCoverforCharacter 0 OpossiteTeam _array_element))
    (CallFunction|ReserveCover _bestcover _array_element)
    (CallFunction|TakeReservedCovers)))

(event EventBeginPlay
  (Utilities|FlowControl|Delay 0.2)
  (Utilities|FlowControl|Sequence
    (:then_0
      (for _array_element (Collision|GetOverlappingActors (Variables|Default|GetBox) "/Game/Blueprints/BP_TestCoverBase.BP_TestCoverBase_C" :!class /Script/Engine.PrimitiveComponent)
        (bind _asbp_test_cover_base (Utilities|Casting|CastToBP_TestCoverBase _array_element))
        (Utilities|Array|Add (Variables|Default|GetCoversInScene) _asbp_test_cover_base)))
    (:then_1
      (for _array_element_2 (Collision|GetOverlappingActors (Variables|Default|GetBox) "/Script/SimpleCoverSystem.AICharacter" :!class /Script/Engine.PrimitiveComponent)
        (bind _asbp_aibase (Utilities|Casting|CastToBP_AIBase _array_element_2))
        (if (Variables|/Game/AI/BP_AIBase.BP_AIBase_C|GetbIsEnemy _asbp_aibase)
          (Utilities|Array|Add (Variables|Default|GetEnemyTeamCharacters) _asbp_aibase)
          (else
            (Utilities|Array|Add (Variables|Default|GetPlayerTeamCharacters) _asbp_aibase)))
        (Utilities|Array|Add (Variables|Default|GetAllAICharacters) _asbp_aibase)))))

(event EventTick
  (params (DeltaSeconds :type Float%20%28single-precision%29)))

(fn ConstructionScript)

(fn FindCoverforCharacter
  (params (TargetEnemy :type BP%20AI%20Base%20Object%20Reference) (EnemyTeam :type Array%20of%20BP%20AI%20Base%20Object%20References) (GivenCharacter :type BP%20AI%20Base%20Object%20Reference))
  (Utilities|FlowControl|Sequence
    (:then_0
      (for _array_element (Variables|Default|GetCoversInScene)
        (if (not (Variables|/Game/Blueprints/BP_TestCoverBase.BP_TestCoverBase_C|GetbIsReserved _array_element))
          (Utilities|Array|Add (LocalVariables|GetCoverCandidates) _array_element)))
      (if (not (> (Utilities|Array|Length (LocalVariables|GetCoverCandidates)) 0))
        (Development|PrintString "Case 0: AllCoversOccupied  -> Return")
        (return false 0 false)))
    (:then_1
      (for _array_element_2 (LocalVariables|GetCoverCandidates)
        (bind _array_element_3 (Utilities|Array|ForEachLoopwithBreak EnemyTeam :!label _label)
          (:LoopBody
            (if (> (Math|Vector|Distance(Vector) (Transformation|GetActorLocation _array_element_3) (Transformation|GetActorLocation _array_element_2)) (Variables|Default|GetMinimumDistanceFromEnemy))
              (Utilities|Array|AddUnique (LocalVariables|GetTempCoverCandidates) _array_element_2)
              (elif (!= (Utilities|Array|FindItem (LocalVariables|GetTempCoverCandidates) _array_element_2) -1)
                (Utilities|Array|RemoveItem (LocalVariables|GetTempCoverCandidates) _array_element_2)
                (goto _label Break)
                (else
                  (goto _label Break)))))))
      (if (<= (Utilities|Array|Length (LocalVariables|GetTempCoverCandidates)) 0)
        (Development|PrintString "Case 1: Covers to close to enemy -> Return")
        (return false 0 false)
        (else
          (if (> (Utilities|Array|Length (LocalVariables|GetTempCoverCandidates)) 1)
            (Development|PrintString (Utilities|String|Append "Case 1: More than 1 cover far enough from the enemy:  " (Utilities|String|ToString(Integer) (Utilities|Array|Length (LocalVariables|GetTempCoverCandidates)))))
            (else
              (Development|PrintString "Case 1: 1 cover far enough from the enemy")))
          (LocalVariables|SetCoverCandidates (LocalVariables|GetTempCoverCandidates))
          (LocalVariables|SetTempCoverCandidates (Utilities|Array|MakeArray)))))
    (:then_2
      (for _array_element_4 (LocalVariables|GetCoverCandidates)
        (bind _array_element_5 (Utilities|Array|ForEachLoopwithBreak EnemyTeam)
          (:LoopBody
            (if (Utilities|Array|ContainsItem (LocalVariables|GetTempCoverCandidates) _array_element_4)
              (Utilities|Array|RemoveItem (LocalVariables|GetTempCoverCandidates) _array_element_4))
            (LocalVariables|SetTargetDirection (.yaw (Math|Rotator|FindRelativeLookatRotation (Transformation|GetWorldTransform (Variables|/Game/Blueprints/BP_TestCoverBase.BP_TestCoverBase_C|GetCoverPosition _array_element_4)) (Transformation|GetActorLocation _array_element_5))))
            (bind _index (Utilities|FlowControl|ForLoopwithBreak 0 3 :!label _label_2)
              (:LoopBody
                (if (Utilities|Select :Index _index :Option%200 (Variables|/Game/Blueprints/BP_TestCoverBase.BP_TestCoverBase_C|GetLeftProtected _array_element_4) :Option%201 (Variables|/Game/Blueprints/BP_TestCoverBase.BP_TestCoverBase_C|GetRightProtected _array_element_4) :Option%202 (Variables|/Game/Blueprints/BP_TestCoverBase.BP_TestCoverBase_C|GetTopProtected _array_element_4) :Option%203 (Variables|/Game/Blueprints/BP_TestCoverBase.BP_TestCoverBase_C|GetBottomProtected _array_element_4))
                  (if (Math|Float|InRange(Float) (LocalVariables|GetTargetDirection) (.value (.lowerbound (Utilities|Select :Index _index :Option%200 (Variables|Default|GetLeftAngleRange) :Option%201 (Variables|Default|GetRightAngleRange) :Option%202 (Variables|Default|GetTopAngleRange) :Option%203 (Variables|Default|GetBottomAngleRange)))) (.value (.upperbound (Utilities|Select :Index _index :Option%200 (Variables|Default|GetLeftAngleRange) :Option%201 (Variables|Default|GetRightAngleRange) :Option%202 (Variables|Default|GetTopAngleRange) :Option%203 (Variables|Default|GetBottomAngleRange)))))
                    (Utilities|Array|AddUnique (LocalVariables|GetTempCoverCandidates) _array_element_4)
                    (goto _label_2 Break))))))))
      (if (<= (Utilities|Array|Length (LocalVariables|GetTempCoverCandidates)) 0)
        (Development|PrintString "Case 2: Can't cover from this enemy -> Return")
        (return false 0 false)
        (elif (> (Utilities|Array|Length (LocalVariables|GetTempCoverCandidates)) 1)
          (Development|PrintString (Utilities|String|Append "Case 2: Found more than 1 safe covers:  " (Utilities|String|ToString(Integer) (Utilities|Array|Length (LocalVariables|GetTempCoverCandidates)))))
          (LocalVariables|SetCoverCandidates (LocalVariables|GetTempCoverCandidates))
          (LocalVariables|SetTempCoverCandidates (Utilities|Array|MakeArray))
          (else
            (Development|PrintString "Case 2: Found one safe cover -> Return")
            (return true (Utilities|Array|Get(acopy) (LocalVariables|GetTempCoverCandidates)) false)))))
    (:then_3
      (Utilities|IsValid TargetEnemy
        (:Is%20Valid
          (for _array_element_6 (LocalVariables|GetCoverCandidates)
            (LocalVariables|SetTargetDirection (.yaw (Math|Rotator|FindRelativeLookatRotation (Transformation|GetWorldTransform (Variables|/Game/Blueprints/BP_TestCoverBase.BP_TestCoverBase_C|GetCoverPosition _array_element_6)) (Transformation|GetActorLocation TargetEnemy))))
            (bind _index_2 (Utilities|FlowControl|ForLoopwithBreak 0 3 :!label _label_3)
              (:LoopBody
                (if (Utilities|Select :Index _index_2 :Option%200 (Variables|/Game/Blueprints/BP_TestCoverBase.BP_TestCoverBase_C|GetLeftProtected _array_element_6) :Option%201 (Variables|/Game/Blueprints/BP_TestCoverBase.BP_TestCoverBase_C|GetRightProtected _array_element_6) :Option%202 (Variables|/Game/Blueprints/BP_TestCoverBase.BP_TestCoverBase_C|GetTopProtected _array_element_6) :Option%203 (Variables|/Game/Blueprints/BP_TestCoverBase.BP_TestCoverBase_C|GetBottomProtected _array_element_6))
                  (if (Math|Float|InRange(Float) (LocalVariables|GetTargetDirection) (+ (.value (.lowerbound (Utilities|Select :Index _index_2 :Option%200 (Variables|Default|GetLeftAngleRange) :Option%201 (Variables|Default|GetRightAngleRange) :Option%202 (Variables|Default|GetTopAngleRange) :Option%203 (Variables|Default|GetBottomAngleRange)))) 15.0) (- (.value (.upperbound (Utilities|Select :Index _index_2 :Option%200 (Variables|Default|GetLeftAngleRange) :Option%201 (Variables|Default|GetRightAngleRange) :Option%202 (Variables|Default|GetTopAngleRange) :Option%203 (Variables|Default|GetBottomAngleRange)))) 15.0))
                    (Utilities|Array|Add (LocalVariables|GetTempCoverCandidates) _array_element_6)
                    (goto _label_3 Break))))))
          (if (<= (Utilities|Array|Length (LocalVariables|GetTempCoverCandidates)) 0)
            (Development|PrintString "Case 3: Can't shoot to this enemy")
            (LocalVariables|SetTempCoverCandidates (Utilities|Array|MakeArray))
            (LocalVariables|SetbCanShootToSelectedEnemy false)
            (elif (> (Utilities|Array|Length (LocalVariables|GetTempCoverCandidates)) 1)
              (Development|PrintString (Utilities|String|Append "Case 3: Found more than one to shoot from:  " (Utilities|String|ToString(Integer) (Utilities|Array|Length (LocalVariables|GetTempCoverCandidates)))))
              (LocalVariables|SetCoverCandidates (LocalVariables|GetTempCoverCandidates))
              (LocalVariables|SetTempCoverCandidates (Utilities|Array|MakeArray))
              (LocalVariables|SetbCanShootToSelectedEnemy true)
              (else
                (Development|PrintString "Case 3: Found one to shoot from -> Return")
                (return true (Utilities|Array|Get(acopy) (LocalVariables|GetTempCoverCandidates)) true)))))))
    (:then_4
      (Utilities|IsValid TargetEnemy
        (:Is%20Valid
          (for _array_element_7 (LocalVariables|GetCoverCandidates)
            (if (<= (Math|Vector|Distance(Vector) (Transformation|GetWorldLocation (Variables|/Game/Blueprints/BP_TestCoverBase.BP_TestCoverBase_C|GetCoverPosition _array_element_7)) (Transformation|GetActorLocation TargetEnemy)) (Variables|Default|GetEffectiveShootDistance))
              (Utilities|Array|Add (LocalVariables|GetTempCoverCandidates) _array_element_7)))
          (if (<= (Utilities|Array|Length (LocalVariables|GetTempCoverCandidates)) 0)
            (Development|PrintString "Case 4: No cover in effective shoot range")
            (elif (> (Utilities|Array|Length (LocalVariables|GetTempCoverCandidates)) 1)
              (Development|PrintString (Utilities|String|Append "Case 4: More than 1 cover in effective shoot range:  " (Utilities|String|ToString(Integer) (Utilities|Array|Length (LocalVariables|GetTempCoverCandidates)))))
              (LocalVariables|SetCoverCandidates (LocalVariables|GetTempCoverCandidates))
              (LocalVariables|SetTempCoverCandidates (Utilities|Array|MakeArray))
              (else
                (Development|PrintString "Case 4: 1 cover in effective shoot range -> Return")
                (return true (Utilities|Array|Get(acopy) (LocalVariables|GetTempCoverCandidates)) true)))))))
    (:then_5
      (LocalVariables|SetIdealCover (Utilities|Array|Get(acopy) (LocalVariables|GetCoverCandidates)))
      (for _array_element_8 (LocalVariables|GetCoverCandidates)
        (if (< (Math|Vector|Distance(Vector) (Transformation|GetWorldLocation (Variables|/Game/Blueprints/BP_TestCoverBase.BP_TestCoverBase_C|GetCoverPosition _array_element_8)) (Transformation|GetActorLocation GivenCharacter)) (Math|Vector|Distance(Vector) (Transformation|GetWorldLocation (Variables|/Game/Blueprints/BP_TestCoverBase.BP_TestCoverBase_C|GetCoverPosition (LocalVariables|GetIdealCover))) (Transformation|GetActorLocation GivenCharacter)))
          (LocalVariables|SetIdealCover _array_element_8)))
      (return true (LocalVariables|GetIdealCover) true))
    (:then_6
      (Development|PrintString (Utilities|String|ToString(Integer) (Utilities|Array|Length (LocalVariables|GetCoverCandidates))) true true "(R=1.000000,G=0.000000,B=0.860542,A=1.000000)"))))