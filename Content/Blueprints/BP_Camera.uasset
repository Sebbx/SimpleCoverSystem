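; Camera Blueprint that serves as a mouse-and-keyboard test controller for the AI cover system, showing the cursor and HUD on BeginPlay.
; Cursor traces on left, right and middle click select a friendly AI, a cover and an enemy, toggling their selection widgets.
; Hotkeys pass these selections to TestCoverSystem to reserve, release, auto-find or take covers, including team-wide assignment.
; A separate debug key prints the best cover from CoverSystem.
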(event EventBeginPlay
  (Variables|/Script/Engine.PlayerController|SetbShowMouseCursor (Game|GetPlayerController 0) true)
  (bind _returnvalue (UserInterface|CreateWidget "/Game/UI/WBP_HUD.WBP_HUD_C"))
  (UserInterface|Viewport|AddtoPlayerScreen _returnvalue))

(event Collision|EventActorBeginOverlap
  (params (OtherActor :type Actor%20Object%20Reference)))

(event EventTick
  (params (DeltaSeconds :type Float%20%28single-precision%29)))

(event Input|KeyboardEvents|3
  (params (Key :type Key%20Structure :default "None"))
  (:Pressed
    (bind (_bestcover _returnvalue) (Class|CoverSystem|FindBestCoverforCharacter (Variables|Default|GetCoverSystem)))
    (Development|PrintString (Utilities|GetDisplayName _bestcover) _returnvalue)))

(event Input|KeyboardEvents|Q
  (params (Key :type Key%20Structure :default "None"))
  (bind _selectedaicharacter (Variables|Default|GetSelectedAICharacter))
  (bind _selectedcover (Variables|Default|GetSelectedCover))
  (:Pressed
    (Utilities|IsValid _selectedaicharacter
      (:Is%20Valid
        (Utilities|IsValid _selectedcover
          (:Is%20Valid
            (Default|ReserveCover (Variables|Default|GetTestCoverSystem) _selectedcover _selectedaicharacter))
          (:Is%20Not%20Valid
            (Development|PrintString "No Cover Selected" true true "(R=1.000000,G=0.000000,B=0.131786,A=1.000000)"))))
      (:Is%20Not%20Valid
        (Development|PrintString "No selected pawn" true true "(R=1.000000,G=0.000000,B=0.131786,A=1.000000)")))))

(event Input|KeyboardEvents|2
  (params (Key :type Key%20Structure :default "None"))
  (bind _testcoversystem (Variables|Default|GetTestCoverSystem))
  (:Pressed
    (Default|FindCoverandReserveforAllCharactersinTeam (Variables|Default|GetTestCoverSystem) (Variables|/Game/Blueprints/BP_TestCoverSystem.BP_TestCoverSystem_C|GetEnemyTeamCharacters _testcoversystem) (Variables|/Game/Blueprints/BP_TestCoverSystem.BP_TestCoverSystem_C|GetPlayerTeamCharacters _testcoversystem))))

(event Input|KeyboardEvents|W
  (params (Key :type Key%20Structure :default "None"))
  (bind _selectedaicharacter (Variables|Default|GetSelectedAICharacter))
  (:Pressed
    (Utilities|IsValid _selectedaicharacter
      (:Is%20Valid
        (Default|DeleteReservation (Variables|Default|GetTestCoverSystem) _selectedaicharacter false))
      (:Is%20Not%20Valid
        (Development|PrintString "No Character Selected" true true "(R=1.000000,G=0.000000,B=0.131786,A=1.000000)")))))

(event Input|MouseEvents|RightMouseButton
  (params (Key :type Key%20Structure :default "None"))
  (:Pressed
    (Utilities|IsValid (Variables|Default|GetSelectedCover)
      (:Is%20Valid
        (Default|DeactivateSelectionWidget (Variables|Default|GetSelectedCover))
        (Variables|Default|SetSelectedCover 0))
      (:Is%20Not%20Valid
        _))
    (bind _asbp_test_cover_base (Utilities|Casting|CastToBP_TestCoverBase (.hitactor (.HitResult (Game|Player|GetHitResultUnderCursorbyChannel (Game|GetPlayerController 0) "TraceTypeQuery1" true)))))
    (bind _output_get (Variables|Default|SetSelectedCover _asbp_test_cover_base))
    (Default|ActivateSelectionWidget _output_get)))

(event Input|KeyboardEvents|E
  (params (Key :type Key%20Structure :default "None"))
  (:Pressed
    (Default|FindandReserveCover (Variables|Default|GetTestCoverSystem) (Variables|Default|GetTargetEnemy) (Variables|Default|GetSelectedAICharacter))))

(event Input|KeyboardEvents|SpaceBar
  (params (Key :type Key%20Structure :default "None"))
  (:Pressed
    (Default|TakeReservedCovers (Variables|Default|GetTestCoverSystem))))

(event Input|MouseEvents|LeftMouseButton
  (params (Key :type Key%20Structure :default "None"))
  (:Pressed
    (Utilities|IsValid (Variables|Default|GetSelectedAICharacter)
      (:Is%20Valid
        (Default|DeactivateCharacterSelectionWidget (Variables|Default|GetSelectedAICharacter))
        (Variables|Default|SetSelectedAICharacter 0))
      (:Is%20Not%20Valid
        _))
    (bind _asbp_aifriendly (Utilities|Casting|CastToBP_AIFriendly (.hitactor (.HitResult (Game|Player|GetHitResultUnderCursorbyChannel (Game|GetPlayerController 0) "TraceTypeQuery1" true)))))
    (bind _output_get (Variables|Default|SetSelectedAICharacter _asbp_aifriendly))
    (Default|ActivateCharacterSelectionWidget _output_get)))

(event Input|MouseEvents|MiddleMouseButton
  (params (Key :type Key%20Structure :default "None"))
  (:Pressed
    (Utilities|IsValid (Variables|Default|GetTargetEnemy)
      (:Is%20Valid
        (Default|DeactivateEnemySelectionWidget (Variables|Default|GetTargetEnemy))
        (Variables|Default|SetTargetEnemy 0))
      (:Is%20Not%20Valid
        _))
    (bind _asbp_aienemy (Utilities|Casting|CastToBP_AIEnemy (.hitactor (.HitResult (Game|Player|GetHitResultUnderCursorbyChannel (Game|GetPlayerController 0) "TraceTypeQuery1" true)))))
    (bind _output_get (Variables|Default|SetTargetEnemy _asbp_aienemy))
    (Default|ActivateEnemySelectionWidget _output_get)))

(event Input|KeyboardEvents|1
  (params (Key :type Key%20Structure :default "None"))
  (bind _testcoversystem (Variables|Default|GetTestCoverSystem))
  (:Pressed
    (Default|FindCoverandReserveforAllCharactersinTeam (Variables|Default|GetTestCoverSystem) (Variables|/Game/Blueprints/BP_TestCoverSystem.BP_TestCoverSystem_C|GetPlayerTeamCharacters _testcoversystem) (Variables|/Game/Blueprints/BP_TestCoverSystem.BP_TestCoverSystem_C|GetEnemyTeamCharacters _testcoversystem))))

(fn ConstructionScript)